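; Enemy turret that tracks the player pawn and fires twin hitscan barrels while the player is within attack range.
; Tick checks distance, eases the guns toward the player with clamped pitch and yaw, then fires through a Delay-based interval.
; Each barrel line-traces from its socket, applying damage and spawning muzzle and impact effects on hits.
; Separate per-barrel aiming events exist but are not wired to run.
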(event Custom|Update%20Range
  ;[1 1 1] Distance to player check
  (if (<= (Transformation|GetDistanceTo self (Game|Player|GetPlayerPawn 0)) (Variables|TurretSettings|GetAttackRange))
    (Variables|Default|SetEnemyInRange true)
    (else
      (Variables|Default|SetEnemyInRange false))))

(event Custom|Update%20Rotation
  (bind _returnvalue (Game|Player|GetPlayerPawn 0))
  (bind _turretguns (Variables|Default|GetTurretGuns))
  (bind _returnvalue_2 (Transformation|GetWorldLocation _turretguns))
  (bind _returnvalue_3 (Transformation|GetActorLocation _returnvalue))
  (bind _returnvalue_4 (Math|Rotator|FindLookatRotation _returnvalue_2 _returnvalue_3))
  (bind (_roll _pitch _yaw) (Math|Rotator|BreakRotator _returnvalue_4))
  ;[1 1 1] Rotation
  (if (Variables|Default|GetEnemyInRange)
    (Transformation|SetWorldRotation (Variables|Default|GetTurretGuns) (Math|Interpolation|RInterpTo (Transformation|GetWorldRotation (Variables|Default|GetTurretGuns)) (Math|Rotator|MakeRotator 0.0 (Math|Float|ClampAngle (- _pitch (Variables|TurretSettings|GetBarrelLength)) -5.0 35.0) (Math|Float|ClampAngle _yaw -1.1e+02 1.1e+02)) (Variables|Default|GetDeltaTime) (Variables|TurretSettings|GetRotationSpeed)) false false)))

(event Custom|Update%20Rotation_Arrow
  (bind _returnvalue (Game|Player|GetPlayerPawn 0))
  (bind _barrel_1 (Variables|Default|GetBarrel_1))
  (bind _returnvalue_2 (Transformation|GetWorldLocation _barrel_1))
  (bind _returnvalue_3 (Transformation|GetActorLocation _returnvalue))
  (bind _returnvalue_4 (Math|Rotator|FindLookatRotation _returnvalue_2 _returnvalue_3))
  (bind (_roll _pitch _yaw) (Math|Rotator|BreakRotator _returnvalue_4))
  ;[1 1 1] Barrel 1 Rotation
  (if (Variables|Default|GetEnemyInRange)
    (Transformation|SetWorldRotation (Variables|Default|GetBarrel_1) (Math|Interpolation|RInterpTo (Transformation|GetWorldRotation (Variables|Default|GetBarrel_1)) (Math|Rotator|MakeRotator 0.0 (Math|Float|ClampAngle (- _pitch (Variables|TurretSettings|GetBarrelLength)) -5.0 35.0) (Math|Float|ClampAngle _yaw -1.1e+02 1.1e+02)) (Variables|Default|GetDeltaTime) (Variables|TurretSettings|GetRotationSpeed)) false false)))

(event Custom|Update%20Rotation_Arrow_2
  (bind _returnvalue (Game|Player|GetPlayerPawn 0))
  (bind _barrel_2 (Variables|Default|GetBarrel_2))
  (bind _returnvalue_2 (Transformation|GetActorLocation _returnvalue))
  (bind _returnvalue_3 (Transformation|GetWorldLocation _barrel_2))
  (bind _returnvalue_4 (Math|Rotator|FindLookatRotation _returnvalue_3 _returnvalue_2))
  (bind (_roll _pitch _yaw) (Math|Rotator|BreakRotator _returnvalue_4))
  ;[1 1 1] Barrel 2 Rotation
  (if (Variables|Default|GetEnemyInRange)
    (Transformation|SetWorldRotation (Variables|Default|GetBarrel_2) (Math|Interpolation|RInterpTo (Transformation|GetWorldRotation (Variables|Default|GetBarrel_2)) (Math|Rotator|MakeRotator 0.0 (Math|Float|ClampAngle (- _pitch (Variables|TurretSettings|GetBarrelLength)) -5.0 35.0) (Math|Float|ClampAngle _yaw -1.1e+02 1.1e+02)) (Variables|Default|GetDeltaTime) (Variables|TurretSettings|GetRotationSpeed)) false false)))

(event Custom|Fire%20Weapons
  (bind _turretguns (Variables|Default|GetTurretGuns))
  (bind _turretguns_2 (Variables|Default|GetTurretGuns))
  (bind _turretguns_3 (Variables|Default|GetTurretGuns))
  (bind _returnvalue (Transformation|GetSocketLocation _turretguns "Barrel_2"))
  (bind _returnvalue_2 (Transformation|GetSocketLocation _turretguns "Barrel_1"))
  (bind _returnvalue_3 (Transformation|GetSocketLocation _turretguns_3 "Barrel_2"))
  (bind _returnvalue_4 (Transformation|GetSocketLocation _turretguns_2 "Barrel_1"))
  ;[1 1 1] Fire Weapons
  (if (Variables|Default|GetEnemyInRange)
    (Utilities|FlowControl|Delay (Variables|TurretSettings|GetFireInterval))
    (Utilities|FlowControl|Sequence
      (:then_0
        (bind (_outhit _returnvalue_5) (Collision|LineTraceByChannel _returnvalue_2 (+ _returnvalue_2 (* (Math|Vector|GetForwardVector (Variables|Default|GetBarrel_1)) (Variables|TurretSettings|GetAttackRange))) "TraceTypeQuery1" false 0 "None"))
        (Utilities|FlowControl|Sequence
          (:then_0
            (if _returnvalue_5
              (bind _output_get (Variables|Default|SetEnd%20Trace (.Location (Collision|BreakHitResult _outhit))))
              (bind _returnvalue_6 (Effects|SpawnEmitteratLocation "/Game/Effects/MuzzleFlash/P_Muzzle_Flash_Infil_Pinch.P_Muzzle_Flash_Infil_Pinch" _returnvalue_4 (Math|Conversions|RotationFromXVector _returnvalue_4)))
              (Game|Damage|ApplyDamage (.HitActor (Collision|BreakHitResult _outhit)) (Variables|TurretSettings|GetBarrelDamage) 0 0)
              (Effects|SpawnEmitteratLocation "/Game/Effects/Impacts/P_Impact_Metal.P_Impact_Metal" _output_get)
              (bind _output_get_2 (Variables|Default|SetMuzzle%20Flash%201 _returnvalue_6))
              (Utilities|FlowControl|Delay 0.1)
              (Components|Activation|Deactivate _output_get_2)
              (if (Variables|Default|GetHit%20Player)
                (Game|Damage|ApplyDamage (stale _aspinch_fpscharacter) (Variables|TurretSettings|GetBarrelDamage) 0 0))
              (else
                (Variables|Default|SetEnd%20Trace "0, 0, 0"))))
          (:then_1
            (bind _aspinch_fpscharacter (Utilities|Casting|CastToPinchFPSCharacter (.HitActor (Collision|BreakHitResult _outhit))))
            (Variables|Default|SetHit%20Player true))))
      (:then_1
        (bind (_outhit_2 _returnvalue_7) (Collision|LineTraceByChannel _returnvalue (+ _returnvalue (* (Math|Vector|GetForwardVector (Variables|Default|GetBarrel_2)) (Variables|TurretSettings|GetAttackRange))) "TraceTypeQuery1" false 0 "None"))
        (Utilities|FlowControl|Sequence
          (:then_0
            (if _returnvalue_7
              (bind _output_get_3 (Variables|Default|SetEnd%20Trace (.Location (Collision|BreakHitResult _outhit_2))))
              (bind _returnvalue_8 (Effects|SpawnEmitteratLocation "/Game/Effects/MuzzleFlash/P_Muzzle_Flash_Infil_Pinch.P_Muzzle_Flash_Infil_Pinch" _returnvalue_3 (Math|Conversions|RotationFromXVector _returnvalue_3)))
              (Game|Damage|ApplyDamage (.HitActor (Collision|BreakHitResult _outhit_2)) (Variables|TurretSettings|GetBarrelDamage) 0 0)
              (Effects|SpawnEmitteratLocation "/Game/Effects/Impacts/P_Impact_Metal.P_Impact_Metal" _output_get_3)
              (bind _output_get_4 (Variables|Default|SetMuzzle%20Flash%202 _returnvalue_8))
              (Utilities|FlowControl|Delay 0.1)
              (Components|Activation|Deactivate _output_get_4)
              (if (Variables|Default|GetHit%20Player)
                (Game|Damage|ApplyDamage 0 (Variables|TurretSettings|GetBarrelDamage) 0 0))
              (else
                (Variables|Default|SetEnd%20Trace "0, 0, 0"))))
          (:then_1
            (Utilities|Casting|CastToPinchFPSCharacter (.HitActor (Collision|BreakHitResult _outhit_2)))
            (Variables|Default|SetHit%20Player true)))))))

(event EventTick
  (params (DeltaSeconds :type Float%20%28single-precision%29))
  ;[1 1 1] Update rotation
  (Variables|Default|SetDeltaTime DeltaSeconds)
  (CallFunction|UpdateRange)
  (CallFunction|UpdateRotation)
  (CallFunction|FireWeapons))

(fn ConstructionScript)