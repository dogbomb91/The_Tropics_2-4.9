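; Test rifle actor that attaches its mesh to a PinchFPSCharacter's rifle component when the character overlaps its trigger.
; FireRifle opens a gate that re-enters itself after a short delay, looping automatic fire with no close in this graph.
; Each shot line-traces from the barrel with debug drawing; hits spawn muzzle flash and metal impact effects and apply damage.
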(event OnComponentBeginOverlap(Trigger)
  (params (OtherActor :type Actor%20Object%20Reference) (OtherComp :type Primitive%20Component%20Object%20Reference) (OtherBodyIndex :type Integer) (bFromSweep :type Boolean) (SweepResult :type Hit%20Result%20Structure%20%28by%20ref%29))
  (bind _aspinch_fpscharacter (Utilities|Casting|CastToPinchFPSCharacter OtherActor))
  (Class|SceneComponent|Attachto (Variables|Default|GetRifle) (Variables|/Game/Blueprints/PinchFPSCharacter.PinchFPSCharacter_C|GetRifle _aspinch_fpscharacter) "None" "KeepRelativeOffset" true))

(event Custom|Fire%20Rifle
  (bind _barrel (Variables|Default|GetBarrel))
  (bind _rifle (Variables|Default|GetRifle))
  (bind _returnvalue (Transformation|GetSocketLocation _rifle "Barrel"))
  (bind _returnvalue_2 (Transformation|GetSocketLocation _barrel "Barrel"))
  (Utilities|FlowControl|Sequence
    (:then_0
      (goto _label Open))
    (:then_1
      (Utilities|FlowControl|Gate true :!label _label
        (:Exit
          (Utilities|FlowControl|Sequence
            (:then_0
              (bind (_outhit _returnvalue_3) (Collision|LineTraceByChannel _returnvalue (+ _returnvalue (* (Math|Vector|GetForwardVector (Variables|Default|GetBarrel)) (Variables|Default|GetMaxShootDist))) "TraceTypeQuery1" false 0 "ForDuration"))
              (if _returnvalue_3
                (bind _output_get (Variables|Default|SetTraceEnd (.Location (Collision|BreakHitResult _outhit))))
                (bind _returnvalue_4 (Effects|SpawnEmitteratLocation "/Game/Effects/MuzzleFlash/P_Muzzle_Flash_Infil_Pinch.P_Muzzle_Flash_Infil_Pinch" _returnvalue_2 (Math|Conversions|RotationFromXVector _returnvalue_2)))
                (Effects|SpawnEmitteratLocation "/Game/Effects/Impacts/P_Impact_Metal.P_Impact_Metal" _output_get)
                (Game|Damage|ApplyDamage (.HitActor (Collision|BreakHitResult _outhit)) (Variables|Default|GetDamage) (Game|GetPlayerController 0) 0)
                (bind _output_get_2 (Variables|Default|SetRifleMuzzleFlash _returnvalue_4))
                (Utilities|FlowControl|Delay 0.1)
                (Components|Activation|Deactivate _output_get_2)
                (else
                  (Variables|Default|SetTraceEnd "0, 0, 0"))))
            (:then_1
              (Utilities|FlowControl|Delay 0.15)
              (goto _label))))))))

(event EventBeginPlay)

(event EventActorBeginOverlap
  (params (OtherActor :type Actor%20Object%20Reference)))

(event EventTick
  (params (DeltaSeconds :type Float%20%28single-precision%29)))

(fn ConstructionScript)