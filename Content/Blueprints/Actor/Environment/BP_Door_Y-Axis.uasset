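; BP_Door_Y-Axis is a sliding door that opens when a PinchFPSCharacter enters its trigger and closes after they leave, both after short delays.
; Timelines drive the slide by adding an offset to the mesh's relative start location, cached at BeginPlay.
; A back trigger, commented as removed but still wired, runs its own timeline only once LeftFront is set by a delay in the front slide's update.
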(event OnComponentBeginOverlap(Trigger)
  (params (OtherActor :type Actor%20Object%20Reference) (OtherComp :type Primitive%20Component%20Object%20Reference) (OtherBodyIndex :type Integer) (bFromSweep :type Boolean) (SweepResult :type Hit%20Result%20Structure%20%28by%20ref%29))
  ;[1 1 1] On overlap with player
  (Utilities|Casting|CastToPinchFPSCharacter OtherActor)
  (Utilities|FlowControl|Delay 0.5)
  ;[1 1 1] Animation for slide
  (bind _slide (Timeline|Slide Play)
    (:Update
      (Transformation|SetRelativeLocation (Variables|Default|GetStaticMesh) (+ _slide (Variables|Default|GetDoorStart)) false false)
      ;[1 1 1] Allow back door to open
      (Utilities|FlowControl|Delay 3.0)
      (Variables|Default|SetLeftFront true))))

(event OnComponentBeginOverlap(BackTrigger)
  (params (OtherActor :type Actor%20Object%20Reference) (OtherComp :type Primitive%20Component%20Object%20Reference) (OtherBodyIndex :type Integer) (bFromSweep :type Boolean) (SweepResult :type Hit%20Result%20Structure%20%28by%20ref%29))
  ;[1 1 1] Back door check (removed)
  (Utilities|Casting|CastToPinchFPSCharacter OtherActor)
  (if (Variables|Default|GetLeftFront)
    (Utilities|FlowControl|Delay 0.5)
    ;[1 1 1] Animation for slide
    (bind _slide (Timeline|Timeline_0 Play)
      (:Update
        (Transformation|SetRelativeLocation (Variables|Default|GetStaticMesh) (+ _slide (Variables|Default|GetDoorStart)) false false)))))

(event OnComponentEndOverlap(BackTrigger)
  (params (OtherActor :type Actor%20Object%20Reference) (OtherComp :type Primitive%20Component%20Object%20Reference) (OtherBodyIndex :type Integer))
  ;[1 1 1] Back door check (removed)
  (Utilities|Casting|CastToPinchFPSCharacter OtherActor)
  (Utilities|FlowControl|Delay 1.5)
  ;[1 1 1] Animation for slide
  (bind _slide (Timeline|Timeline_0 Reverse)
    (:Update
      (Transformation|SetRelativeLocation (Variables|Default|GetStaticMesh) (+ _slide (Variables|Default|GetDoorStart)) false false))))

(event OnComponentEndOverlap(Trigger)
  (params (OtherActor :type Actor%20Object%20Reference) (OtherComp :type Primitive%20Component%20Object%20Reference) (OtherBodyIndex :type Integer))
  ;[1 1 1] On overlap with player
  (Utilities|Casting|CastToPinchFPSCharacter OtherActor)
  (Utilities|FlowControl|Delay 1.5)
  ;[1 1 1] Animation for slide
  (bind _slide (Timeline|Slide Reverse)
    (:Update
      (Transformation|SetRelativeLocation (Variables|Default|GetStaticMesh) (+ _slide (Variables|Default|GetDoorStart)) false false)
      ;[1 1 1] Allow back door to open
      (Utilities|FlowControl|Delay 3.0)
      (Variables|Default|SetLeftFront true))))

(event EventBeginPlay
  ;[1 1 1] Get initial location
  (Variables|Default|SetDoorStart (Variables|/Script/Engine.SceneComponent|GetRelativeLocation (Variables|Default|GetStaticMesh))))

(fn ConstructionScript)