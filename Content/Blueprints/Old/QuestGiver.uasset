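; Quest giver Blueprint that offers a quest to the player through a widget when they enter its trigger.
; On overlap by the PinchFPSCharacter, it creates a new QuestWidget and shows the mouse cursor, unless the stored widget's HasAccepted flag is set.
; Leaving the trigger before accepting removes all widgets on screen, not just the quest one, and hides the cursor.
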(event OnComponentBeginOverlap(Trigger)
  (params (OtherActor :type Actor%20Object%20Reference) (OtherComp :type Primitive%20Component%20Object%20Reference) (OtherBodyIndex :type Integer) (bFromSweep :type Boolean) (SweepResult :type Hit%20Result%20Structure%20%28by%20ref%29))
  (bind _returnvalue (Game|GetPlayerController 0))
  (Utilities|Casting|CastToPinchFPSCharacter OtherActor)
  (if (not (Variables|/Game/Blueprints/Old/QuestWidget.QuestWidget_C|GetHas%20Accepted (stale _returnvalue_2)))
    (bind _returnvalue_2 (UserInterface|CreateWidget "/Game/Blueprints/Old/QuestWidget.QuestWidget_C" _returnvalue))
    (UserInterface|Viewport|AddtoViewport _returnvalue_2 0)
    (Variables|/Script/Engine.PlayerController|SetbShowMouseCursor _returnvalue true)))

(event OnComponentEndOverlap(Trigger)
  (params (OtherActor :type Actor%20Object%20Reference) (OtherComp :type Primitive%20Component%20Object%20Reference) (OtherBodyIndex :type Integer))
  (Utilities|Casting|CastToPinchFPSCharacter OtherActor)
  (if (not (Variables|/Game/Blueprints/Old/QuestWidget.QuestWidget_C|GetHas%20Accepted (stale OnComponentBeginOverlap(Trigger) _returnvalue_2)))
    (Viewport|RemoveAllWidgets)
    (Variables|/Script/Engine.PlayerController|SetbShowMouseCursor (Game|GetPlayerController 0) false)))

(fn ConstructionScript)